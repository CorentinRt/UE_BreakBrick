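; BP_Player_BB is a player Blueprint that adds a timed "reduce" effect, shrinking the actor along its Y scale.
; A start event flags the effect active and records the start time.
; Each Tick, after the parent's, an update clears the flag once the duration elapses and uses FInterpTo to ease Y scale toward the reduced target or back to 1, leaving X and Z untouched.
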(event `CE_StartReducePlayerEffect`
  ;[0.8524 0.7581 0.2139 0.5] Start Reduce Player Effect
  (`|ExecutionSequence`
    (:`then_0`
      (set `self.bIsReducing` true))
    (:`then_1`
      (set `self.StartReducingTime` (`GameplayStatics.GetTimeSeconds`)))))

(event `CE_UpdateReducingPlayer`
  (params (InDeltaTime :type "Float (double-precision)"))
  (bind (_returnvalue_x _returnvalue_y _returnvalue_z) (`KismetMathLibrary.BreakVector` (`self.GetActorScale3D`)))
  ;[0.8906 0.4482 0.2727 0.5] Update ReducingPlayer
  (`|ExecutionSequence`
    (:`then_0`
      (if (>= (- (`GameplayStatics.GetTimeSeconds`) (`self.StartReducingTime`)) (`self.ReducingTotalDuration`))
        (set `self.bIsReducing` false)))
    (:`then_1`
      (`self.SetActorScale3D` (`KismetMathLibrary.MakeVector` _returnvalue_x (`KismetMathLibrary.FInterpTo` _returnvalue_y (`KismetMathLibrary.SelectFloat` (`self.ReducingTargetScale`) 1.0 (`self.bIsReducing`)) InDeltaTime (`self.ReducingSpeed`)) _returnvalue_z)))))

(event `self.ReceiveTick`
  (params (DeltaSeconds :type "Float (single-precision)"))
  ;[0.9253 0.2018 0.1221 0.5] Tick
  (`parent.ReceiveTick` DeltaSeconds)
  (`|ExecutionSequence`
    (:`then_0`
      (`self.CE_UpdateReducingPlayer` DeltaSeconds))))

(fn `UserConstructionScript`)