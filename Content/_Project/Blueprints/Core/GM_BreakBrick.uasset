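; Game mode for a brick-breaker game that runs the flow of rounds and the end of the game.
; It starts rounds with a countdown sound and delayed ball launch, then on round or game end clears balls and bricks through world subsystems and plays result sounds.
; It also crossfades music, blends the view to the main camera, shakes it when bricks break, and saves new high scores to a save slot.
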(event `CE_LoadSaveGameDatas`
  ;[0.2115 0.7695 0.842 0.5] Load Save Game Datas
  (bind _returnvalue (`GameplayStatics.DoesSaveGameExist` (`self.SaveGameName`)))
  (if _returnvalue
    (bind _returnvalue_2 (`GameplayStatics.LoadGameFromSlot` (`self.SaveGameName`)))
    (bind _asbp_save_game_datas (cast `/Game/_Project/Blueprints/SaveGame/BP_SaveGameDatas` _returnvalue_2))
    (set `self.SaveGameDatas` _asbp_save_game_datas)
    (else
      (bind _returnvalue_3 (`GameplayStatics.CreateSaveGameObject` "/Game/_Project/Blueprints/SaveGame/BP_SaveGameDatas.BP_SaveGameDatas_C"))
      (set `self.SaveGameDatas` _returnvalue_3))))

(event `CE_SwitchCurrentMusic`
  (params (InSound :type "SoundBase Object Reference") (InFadeIn :type "Float (double-precision)") (InFadeOut :type "Float (double-precision)"))
  (bind _musicaudiocomponent (`self.MusicAudioComponent`))
  ;[0.7655 0.2521 0.8837 0.5] Switch Current Music
  (`self.MusicAudioComponent`
    (:`then`
      (`|ExecutionSequence`
        (:`then_0`
          (`AudioComponent.FadeOut` _musicaudiocomponent InFadeOut 0.0 "Linear"))
        (:`then_1`
          (`KismetSystemLibrary.Delay` InFadeOut)
          (`AudioComponent.SetSound` _musicaudiocomponent InSound)
          (`AudioComponent.FadeIn` _musicaudiocomponent InFadeIn 1.0 0.0 "Linear"))))
    (:`else`
      (bind _returnvalue (`GameplayStatics.SpawnSound2D` InSound 1.0 1.0 0.0 null false false))
      (bind _output_get (set `self.MusicAudioComponent` _returnvalue))
      (`AudioComponent.FadeIn` _output_get InFadeIn 1.0 0.0 "Linear"))))

(event `CE_SetHighScore`
  (params (InHighScore :type Integer))
  ;[0.2115 0.7695 0.842 0.5] Load Save Game Datas
  (`|ExecutionSequence`
    (:`then_0`
      (bind _savegamedatas (`self.SaveGameDatas`)
        (:`then`
          (set `/Game/_Project/Blueprints/SaveGame/BP_SaveGameDatas.HighScore` InHighScore _savegamedatas)
          (`GameplayStatics.SaveGameToSlot` (`self.SaveGameDatas`) (`self.SaveGameName`) :!label _label))
        (:`else`
          (`self.CE_LoadSaveGameDatas`))))
    (:`then_1`
      (bind _savegamedatas_2 (`self.SaveGameDatas`)
        (:`then`
          (set `/Game/_Project/Blueprints/SaveGame/BP_SaveGameDatas.HighScore` InHighScore _savegamedatas_2)
          (goto _label))
        (:`else`)))))

(event `self.ReceiveStartGame`
  ;[0.1738 0.4734 0.9219 0.5] Receive Start Game
)

(event `CE_SetBlendViewToMainCamera`
  (bind _returnvalue (`GameplayStatics.GetPlayerController` 0))
  (bind _returnvalue_2 (subsystem `CameraWorldSubsystem`))
  ;[0.2719 0.9774 0.4747 0.5] Set Blend View To Main Camera
  (`/Engine/EditorBlueprintResources/StandardMacros.IsValid` _returnvalue_2
    (:`Is Valid`
      (bind _camera (`CameraWorldSubsystem.Camera` _returnvalue_2)
        (:`then`
          (`/Engine/EditorBlueprintResources/StandardMacros.IsValid` _returnvalue
            (:`Is Valid`
              (`PlayerController.SetViewTargetWithBlend` _returnvalue _camera 0.0 "VTBlend_Linear" 0.0 false))))
        (:`else`)))))

(event `self.ReceiveInitSubsystems`
  ;[0.1201 0.9219 0.6365 0.5] Receive Init subsystems
  (`|ExecutionSequence`
    (:`then_0`
      (`self.CE_SetBlendViewToMainCamera`))
    (:`then_1`
      (`self.CE_StartGameAndLaunchBallAfterDelay` 1.3 2.0))
    (:`then_2`
      (`self.F_GetPlayerPawn`))
    (:`then_3`
      (`self.CE_LoadSaveGameDatas`))))

(event `CE_StartGameAndLaunchBallAfterDelay`
  (params (InLaunchBallDelay :type "Float (double-precision)") (InPreSoundDelay :type "Float (double-precision)"))
  ;[0.3388 0.9166 0.9219 0.5] Start Game And launch Ball After Delay
  (bind _returnvalue (`self.StartGame` true))
  (`|ExecutionSequence`
    (:`then_0`
      (`KismetSystemLibrary.Delay` InPreSoundDelay)
      (`GameplayStatics.PlaySound2D` "/Game/_Project/Audio/MUS/MS_MUS_InGame_321.MS_MUS_InGame_321" 1.0 1.0 0.0 null self)
      (`KismetSystemLibrary.Delay` InLaunchBallDelay)
      (`|ExecutionSequence`
        (:`then_0`
          (`/Engine/EditorBlueprintResources/StandardMacros.IsValid` _returnvalue
            (:`Is Valid`
              (`Ball_BB.Init` _returnvalue))))
        (:`then_1`
          (`self.CE_SwitchCurrentMusic` "/Game/_Project/Audio/MUS/MS_MUS_InGame_Main.MS_MUS_InGame_Main"))))
    (:`then_1`
      (bind _outplayerpawn (`self.F_GetPlayerPawn`))
      (`/Engine/EditorBlueprintResources/StandardMacros.IsValid` _outplayerpawn
        (:`Is Valid`
          (`/Game/_Project/Blueprints/Player/BP_Player_BB.CE_DisplayTutoInput` _outplayerpawn))))))

(event `self.ReceiveRoundFinished`
  (params (InRoundFinishedID :type "ERoundFinishedID Enum" :default "ALL_BRICKS_DESTROYED"))
  ;[0.3997 0.3164 0.9219 0.5] Receive Round Finished
  (`self.CE_ClearBothBallsAndBricks`)
  (switch `ERoundFinishedID` InRoundFinishedID
    (:`ALL_BRICKS_DESTROYED`
      (`self.CE_HandleRoundVictory`))
    (:`ALL_BALLS_DESTROYED`
      (`self.CE_HandleRoundDefeat`))))

(event `CE_ClearBothBallsAndBricks`
  (bind _returnvalue (subsystem `BricksWallWorldSubsystem`))
  (bind _returnvalue_2 (subsystem `BallsWorldSubsystem`))
  ;[0.9531 0.742 0.166 0.5] Clear Both balls and bricks
  (`|ExecutionSequence`
    (:`then_0`
      (`/Engine/EditorBlueprintResources/StandardMacros.IsValid` _returnvalue
        (:`Is Valid`
          (`BricksWallWorldSubsystem.ClearBricksWall` _returnvalue))))
    (:`then_1`
      (`/Engine/EditorBlueprintResources/StandardMacros.IsValid` _returnvalue_2
        (:`Is Valid`
          (`BallsWorldSubsystem.ClearBalls` _returnvalue_2))))))

(event `self.ReceiveGameFinished`
  (params (InGameFinishedID :type "EGameFinishedID Enum" :default "DEFEAT"))
  ;[0.3997 0.3164 0.9219 0.5] Receive Game Finished
  (`self.CE_ClearBothBallsAndBricks`)
  (switch `EGameFinishedID` InGameFinishedID
    (:`DEFEAT`
      (`self.CE_HandleDefeat`))
    (:`VICTORY`
      (`self.CE_HandleVictory`))))

(event `CE_HandleVictory`
  ;[0.8976 0.7906 0.3079 0.5] Handle Game Victory Defeat
  (`KismetSystemLibrary.PrintString` "GAME VICTORY !!!" true true (struct :`R` 1.0 :`G` 0.898794 :`A` 1.0))
  (set `self.bIsGameFinished` true :!label _label_2)
  (`self.CE_HandleNewHighScorePossibility`)
  (`GameplayStatics.PlaySound2D` "/Game/_Project/Audio/SFX/VictoryDefeat/MS_SFX_EndGame.MS_SFX_EndGame" 2.0 1.0 0.0 null null)
  (`self.CE_SwitchCurrentMusic` "/Game/_Project/Audio/MUS/MS_MUS_InGame_Waiting.MS_MUS_InGame_Waiting" 0.3 0.5))

(event `CE_HandleRoundVictory`
  ;[0.8976 0.7906 0.3079 0.5] Handle Round Victory Defeat
  (`KismetSystemLibrary.PrintString` "ROUND VICTORY !!!" true true (struct :`R` 1.0 :`G` 0.898794 :`A` 1.0))
  (`GameplayStatics.PlaySound2D` "/Game/_Project/Audio/SFX/VictoryDefeat/MS_SFX_Victory.MS_SFX_Victory" 2.0 1.0 0.0 null self)
  (`self.IncrementCurrentLevel`)
  (`self.CE_SwitchCurrentMusic` "/Game/_Project/Audio/MUS/MS_MUS_InGame_Waiting.MS_MUS_InGame_Waiting" 0.3 0.5 :!label _label_3)
  (`KismetSystemLibrary.Delay` 3.0)
  (`self.CE_StartGameAndLaunchBallAfterDelay` 1.3 1.5))

(event `CE_PlayBrickDestructCameraShake`
  (bind _returnvalue (subsystem `CameraWorldSubsystem`))
  ;[0.8389 0.2531 0.9323 0.5] Play Brick Destruct Camera Shake
  (`/Engine/EditorBlueprintResources/StandardMacros.IsValid` _returnvalue
    (:`Is Valid`
      (`|ExecutionSequence`
        (:`then_0`
          (`CameraWorldSubsystem.PlayCameraShake` _returnvalue (`self.ShakeBrickDestruct`) 1.0))))))

(event `self.ReceiveOneBrickDestruct`
  (params (InBrick :type "Brick_Base Object Reference"))
  ;[0.8602 0.1745 0.8767 0.5] Receive One Brick Destruct
  (`/Engine/EditorBlueprintResources/StandardMacros.IsValid` InBrick
    (:`Is Valid`
      (`|ExecutionSequence`
        (:`then_0`
          (`self.CE_PlayBrickDestructCameraShake`))))))

(event `CE_HandleRoundDefeat`
  ;[0.8976 0.7906 0.3079 0.5] Handle Round Victory Defeat
  (`KismetSystemLibrary.PrintString` "ROUND DEFEAT !!!" true true (struct :`R` 1.0 :`G` 0.898794 :`A` 1.0))
  (`GameplayStatics.PlaySound2D` "/Game/_Project/Audio/SFX/VictoryDefeat/MS_SFX_Defeat.MS_SFX_Defeat" 2.0 1.0 0.0 null self)
  (goto _label_3))

(event `CE_HandleDefeat`
  ;[0.8976 0.7906 0.3079 0.5] Handle Game Victory Defeat
  (`KismetSystemLibrary.PrintString` "GAME DEFEAT !!!" true true (struct :`R` 1.0 :`G` 0.898794 :`A` 1.0))
  (goto _label_2))

(event `CE_HandleNewHighScorePossibility`
  (bind _returnvalue (subsystem `ScoreWorldSubsystem`))
  (bind _returnvalue_2 (`ScoreWorldSubsystem.GetScore` _returnvalue))
  ;[0.1057 0.8139 0.8906 0.5] Handle new high score possibility
  (`/Engine/EditorBlueprintResources/StandardMacros.IsValid` _returnvalue
    (:`Is Valid`
      (bind _outhighscore (`self.F_GetHighScore`))
      (if (> _returnvalue_2 _outhighscore)
        (`self.CE_SetHighScore` _returnvalue_2)
        (`self.ED_OnSetNewHighScore` _returnvalue_2)))))

(fn `F_GetHighScore`
  (returns (OutHighScore :type Integer))
  (`|ExecutionSequence`
    (:`then_0`
      (bind _savegamedatas (`self.SaveGameDatas`)
        (:`then`
          (return (`/Game/_Project/Blueprints/SaveGame/BP_SaveGameDatas.HighScore` _savegamedatas)))
        (:`else`
          (`self.CE_LoadSaveGameDatas`))))
    (:`then_1`
      (bind _savegamedatas_2 (`self.SaveGameDatas`)
        (:`then`
          (return (`/Game/_Project/Blueprints/SaveGame/BP_SaveGameDatas.HighScore` _savegamedatas_2)))
        (:`else`
          (return 0))))))

(fn `F_GetPlayerPawn`
  (returns (OutPlayerPawn :type "/Game/_Project/Blueprints/Player/BP_Player_BB Object Reference"))
  (bind _playerpawn (`self.PlayerPawn`)
    (:`then`
      (return _playerpawn))
    (:`else`
      (bind _asbp_player_bb (cast `/Game/_Project/Blueprints/Player/BP_Player_BB` (`GameplayStatics.GetPlayerPawn` 0))
        (:`then`
          (bind _output_get (set `self.PlayerPawn` _asbp_player_bb))
          (return _output_get))
        (:`CastFailed`
          (return null))))))

(fn `UserConstructionScript`)