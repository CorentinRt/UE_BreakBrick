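; Ball actor that bounces, flashes and pulses on impact, and destroys destructible objects it hits.
; Sphere collision hits trigger the bounce and message non-ball actors implementing the Destructible interface.
; On bounce, a half-second linear tween samples curves to drive emissive on a dynamic material instance and mesh scale relative to its original.
; BeginPlay creates that material, caches the scale and gives the Niagara trail absolute rotation.
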(event `CE_CreateBallMaterial`
  (bind _staticmesh (`self.StaticMesh`))
  ;[0.3994 0.7865 0.5281 0.5] Create Ball Material
  (bind _returnvalue (`PrimitiveComponent.CreateDynamicMaterialInstance` _staticmesh 0 "/Game/_Project/Art/Materials/Ball/MI_Ball.MI_Ball" "None"))
  (bind _output_get (set `self.BallMaterialInstance` _returnvalue))
  (`PrimitiveComponent.SetMaterial` _staticmesh 0 _output_get))

(event `self.ReceiveOnBounced`
  ;[0.8906 0.2752 0.6846 0.5] Receive On Bounced
  (`|ExecutionSequence`
    (:`then_0`
      (bind (_asynctaskproxy _value) (`FCTweenBPActionFloat.TweenFloat` 0.0 1.0 0.5 "Linear")
        (:`ApplyEasing`
          (`|ExecutionSequence`
            (:`then_0`
              (bind _emissivecurve (`self.EmissiveCurve`)
                (:`then`
                  (bind _ballmaterialinstance (`self.BallMaterialInstance`)
                    (:`then`
                      (`MaterialInstanceDynamic.SetScalarParameterValue` _ballmaterialinstance (`self.AlphaEmissiveParameterName`) (`CurveFloat.GetFloatValue` _emissivecurve _value)))
                    (:`else`)))
                (:`else`)))
            (:`then_1`
              (bind _scalecurve (`self.ScaleCurve`)
                (:`then`
                  (bind _staticmesh (`self.StaticMesh`)
                    (:`then`
                      (`SceneComponent.SetRelativeScale3D` _staticmesh (* (`CurveFloat.GetFloatValue` _scalecurve _value) (`self.OriginScale`))))
                    (:`else`)))
                (:`else`)))))))))

(event `self.ReceiveBeginPlay`
  ;[0.3348 0.9149 0.3972 0.5] Begin Play
  (`|ExecutionSequence`
    (:`then_0`
      (`self.CE_CreateBallMaterial`))
    (:`then_1`
      (bind _staticmesh (`self.StaticMesh`)
        (:`then`
          (set `self.OriginScale` (`SceneComponent.RelativeScale3D` _staticmesh)))
        (:`else`)))
    (:`then_2`
      (set `SceneComponent.bAbsoluteRotation` true (`self.NS_Ball_Trail`)))))

(event `self.SphereCollision.OnComponentHit`
  (params (HitComponent :type "PrimitiveComponent Object Reference") (OtherActor :type "Actor Object Reference") (OtherComp :type "PrimitiveComponent Object Reference") (NormalImpulse :type "Vector Structure") (Hit :type "HitResult Structure (by ref)"))
  ;[0.9184 0.0988 0.01418 0.5] On Sphere Collision Hit
  (`/Engine/EditorBlueprintResources/StandardMacros.IsValid` OtherActor
    (:`Is Valid`
      (`|ExecutionSequence`
        (:`then_0`
          (`Bouncable.Bounced`))
        (:`then_1`
          (if (not (`self.ActorHasTag` OtherActor (`self.BallTag`)))
            (if (`KismetSystemLibrary.DoesImplementInterface` OtherActor "/Script/BreakBrick.Destructible")
              (message `Destructible.Destruct` OtherActor))))))))

(fn `UserConstructionScript`)