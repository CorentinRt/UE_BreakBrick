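; Brick Blueprint that triggers a reduce-player effect on the player when destroyed.
; It caches the player pawn as BP_Player_BB on BeginPlay.
; On destruct it requests that effect from the player unless the bricks wall subsystem reports all bricks destroyed, then hides its icon widget, plays a 2D sound and calls the parent's destruct logic.
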(event `self.ReceiveBeginPlay`
  (bind _returnvalue (`GameplayStatics.GetPlayerPawn` 0))
  ;[0.2615 0.8559 0.3003 0.5] Begin Play
  (`parent.ReceiveBeginPlay`)
  (`|ExecutionSequence`
    (:`then_0`
      (`/Engine/EditorBlueprintResources/StandardMacros.IsValid` _returnvalue
        (:`Is Valid`
          (bind _asbp_player_bb (cast `/Game/_Project/Blueprints/Player/BP_Player_BB` _returnvalue))
          (set `self.Player` _asbp_player_bb))))))

(event `CE_RequestReducePlayerEffect`
  (bind _returnvalue (subsystem `BricksWallWorldSubsystem`))
  ;[0.215 0.5737 0.8698 0.5] Request Reduce Player Effect
  (`|ExecutionSequence`
    (:`then_0`
      (`/Engine/EditorBlueprintResources/StandardMacros.IsValid` _returnvalue
        (:`Is Valid`
          (if (not (`BricksWallWorldSubsystem.AllBricksAreDestroyed` _returnvalue))
            (bind _player (`self.Player`)
              (:`then`
                (`/Game/_Project/Blueprints/Player/BP_Player_BB.CE_StartReducePlayerEffect` _player))
              (:`else`))))))))

(event `self.ReceiveOnDestruct`
  ;[0.9323 0.1387 0.2019 0.5] Receive On Destruct
  (`|ExecutionSequence`
    (:`then_0`
      (`self.CE_RequestReducePlayerEffect`)
      (bind _widget_icon (`self.Widget_Icon`)
        (:`then`
          (`SceneComponent.SetVisibility` _widget_icon false false))
        (:`else`)))
    (:`then_1`
      (`GameplayStatics.PlaySound2D` "/Game/_Project/Audio/SFX/Bricks/ReducePlayer/MS_SFX_ReducePlayer.MS_SFX_ReducePlayer" 2.0 1.0 0.0 null null))
    (:`then_2`
      (`parent.ReceiveOnDestruct`))))

(fn `UserConstructionScript`
  (`parent.UserConstructionScript`))