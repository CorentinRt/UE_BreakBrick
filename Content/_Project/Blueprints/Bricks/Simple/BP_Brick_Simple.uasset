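; Simple brick that plays effects and an animated exit when destructed.
; On destruct it plays sound, Niagara explosion and force feedback, and spawns a score actor when its data gives a nonzero score.
; Unless flagged for immediate destruction, it disables collision and runs a curve-driven tween on mesh offset, scale (via CurveRotation) and dynamic-material emissive, then destroys itself.
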(event `CE_CreateMaterialInstanceBrick`
  (bind _brickmesh (`self.BrickMesh`))
  ;[0.3287 0.8559 0.7294 0.5] Create Material Instance Brick
  (bind _returnvalue (`PrimitiveComponent.CreateDynamicMaterialInstance` _brickmesh 0 (`PrimitiveComponent.GetMaterial` (`self.BrickMesh`) 0) "None"))
  (bind _output_get (set `self.BrickMaterial` _returnvalue))
  (`PrimitiveComponent.SetMaterial` _brickmesh 0 _output_get))

(event `self.ReceiveBeginPlay`
  ;[0.2717 0.8976 0.4444 0.5] Begin Play
  (`|ExecutionSequence`
    (:`then_0`
      (`self.CE_CreateMaterialInstanceBrick`))
    (:`then_1`
      (bind _brickmesh (`self.BrickMesh`)
        (:`then`
          (set `self.OriginalScale` (`SceneComponent.RelativeScale3D` _brickmesh)))
        (:`else`)))))

(event `CE_PlayDestructEffects`
  (bind _returnvalue (`GameplayStatics.GetPlayerController` 0))
  ;[0.7732 0.1689 0.9531 0.5] Play Destruct Effects
  (`|ExecutionSequence`
    (:`then_0`
      (`self.CE_SpawnScoreEffect`))
    (:`then_1`
      (`GameplayStatics.PlaySound2D` "/Game/_Project/Audio/SFX/Bricks/Destruct/MS_SFX_Brick_Destruct.MS_SFX_Brick_Destruct" 1.0 1.0 0.0 null self))
    (:`then_2`
      (`NiagaraFunctionLibrary.SpawnSystemAtLocation` "/Game/_Project/Art/VFX/Bricks/NS_Brick_Explosion.NS_Brick_Explosion" (`self.K2_GetActorLocation`)))
    (:`then_3`
      (`/Engine/EditorBlueprintResources/StandardMacros.IsValid` _returnvalue
        (:`Is Valid`
          (`PlayerController.K2_ClientPlayForceFeedback` _returnvalue "/Game/_Project/Datas/ForceFeedbacks/FFE_BrickDestruct.FFE_BrickDestruct" "None" false false false))))))

(event `CE_SpawnScoreEffect`
  ;[0.8722 0.3973 0.8837 0.5] Spawn Score Effect
  (bind _datas (`self.Datas`)
    (:`then`
      (bind _scoreondestruct (`BrickDatas_Base.ScoreOnDestruct` _datas))
      (if (!= _scoreondestruct 0.0)
        (bind _returnvalue (`|SpawnActorFromClass` "/Game/_Project/Blueprints/Bricks/Score/BP_Brick_Score.BP_Brick_Score_C" (`KismetMathLibrary.MakeTransform` (+ (`self.K2_GetActorLocation`) (`KismetMathLibrary.MakeVector` (+ -100.0 (`KismetMathLibrary.RandomFloat`))))) "AlwaysSpawn" "MultiplyWithRoot" null null))
        (`/Game/_Project/Blueprints/Bricks/Score/BP_Brick_Score.CE_Init` _returnvalue (`KismetMathLibrary.FTrunc` _scoreondestruct))))
    (:`else`)))

(event `self.ReceiveOnDestruct`
  ;[0.9323 0.1387 0.2019 0.5] Receive On Destruct
  (`|ExecutionSequence`
    (:`then_0`
      (`self.CE_PlayDestructEffects`))
    (:`then_1`
      (`self.bDestroyImmediatlyOnDestruct`
        (:`then`)
        (:`else`
          (`self.CE_CustomHandlingDestruct`))))))

(event `CE_CustomHandlingDestruct`
  ;[0.9045 0.2536 0.1304 0.5] Custom Handling Destruct
  (`|ExecutionSequence`
    (:`then_0`
      (`PrimitiveComponent.SetCollisionEnabled` (`self.BoxCollision`) "NoCollision"))
    (:`then_1`
      (bind (_asynctaskproxy _value) (`FCTweenBPActionFloat.TweenFloat` 0.0 1.0 0.5 "Linear")
        (:`ApplyEasing`
          (`|ExecutionSequence`
            (:`then_0`
              (bind _curveoffset (`self.CurveOffset`)
                (:`then`
                  (bind _brickmesh (`self.BrickMesh`)
                    (:`then`
                      (bind _returnvalue (`CurveFloat.GetFloatValue` _curveoffset _value))
                      (`SceneComponent.K2_SetRelativeLocation` _brickmesh (`KismetMathLibrary.MakeVector` 0.0 (* _returnvalue -7.0) (* _returnvalue 7.0)) false false))
                    (:`else`)))
                (:`else`)))
            (:`then_1`
              (bind _curveemissive (`self.CurveEmissive`)
                (:`then`
                  (bind _brickmaterial (`self.BrickMaterial`)
                    (:`then`
                      (`MaterialInstanceDynamic.SetScalarParameterValue` _brickmaterial (`self.AlphaEmissiveParameterName`) (`CurveFloat.GetFloatValue` _curveemissive _value)))
                    (:`else`)))
                (:`else`)))
            (:`then_2`
              (bind _curverotation (`self.CurveRotation`)
                (:`then`
                  (bind _brickmesh_2 (`self.BrickMesh`)
                    (:`then`
                      (`SceneComponent.SetRelativeScale3D` _brickmesh_2 (* (`CurveFloat.GetFloatValue` _curverotation _value) (`self.OriginalScale`))))
                    (:`else`)))
                (:`else`)))))
        (:`OnComplete`
          (`/Engine/EditorBlueprintResources/StandardMacros.IsValid` self
            (:`Is Valid`
              (`self.K2_DestroyActor`))))))))

(fn `UserConstructionScript`)