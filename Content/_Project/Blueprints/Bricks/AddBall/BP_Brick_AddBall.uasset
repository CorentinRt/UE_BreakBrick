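; BP_Brick_AddBall is a brick that grants an extra ball when it is destroyed.
; On destruct it fires an add-ball request, then runs the parent destruct logic.
; The request asks the balls world subsystem to create a new ball only if the bricks wall subsystem reports that bricks still remain.
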(event `CE_RequestAddNewBallEffect`
  (bind _returnvalue (subsystem `BallsWorldSubsystem`))
  (bind _returnvalue_2 (subsystem `BricksWallWorldSubsystem`))
  ;[0.215 0.5737 0.8698 0.5] Request Add new Ball Effect
  (`|ExecutionSequence`
    (:`then_0`
      (`/Engine/EditorBlueprintResources/StandardMacros.IsValid` _returnvalue_2
        (:`Is Valid`
          (if (not (`BricksWallWorldSubsystem.AllBricksAreDestroyed` _returnvalue_2))
            (`/Engine/EditorBlueprintResources/StandardMacros.IsValid` _returnvalue
              (:`Is Valid`
                (`BallsWorldSubsystem.CreateNewBall` _returnvalue true)))))))))

(event `self.ReceiveOnDestruct`
  ;[0.9323 0.1387 0.2019 0.5] Receive On Destruct
  (`|ExecutionSequence`
    (:`then_0`
      (`self.CE_RequestAddNewBallEffect`))
    (:`then_1`
      (`parent.ReceiveOnDestruct`))))

(fn `UserConstructionScript`
  (`parent.UserConstructionScript`))